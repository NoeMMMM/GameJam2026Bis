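; BP_Pompe is an interactable pump that animates its two handle parts when the player presses E nearby.
; A trigger overlap enables input and shows a prompt widget, and leaving it reverses both.
; One timeline lerps the handles from their BeginPlay positions by a Decrease offset, then a second timeline returns them.
; The Isanimated flag is never reset here, so the stroke plays only once.
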(event OnComponentBeginOverlap(Trigger)
  (params (OverlappedComponent :type Primitive%20Component%20Object%20Reference) (OtherActor :type Actor%20Object%20Reference) (OtherComp :type Primitive%20Component%20Object%20Reference) (OtherBodyIndex :type Integer) (bFromSweep :type Boolean) (SweepResult :type Hit%20Result%20Structure%20%28by%20ref%29))
  (Input|EnableInput (Game|GetPlayerController 0))
  (Rendering|SetVisibility (Variables|Default|GetWidget) true false))

(event OnComponentEndOverlap(Trigger)
  (params (OverlappedComponent :type Primitive%20Component%20Object%20Reference) (OtherActor :type Actor%20Object%20Reference) (OtherComp :type Primitive%20Component%20Object%20Reference) (OtherBodyIndex :type Integer))
  (Input|DisableInput (Game|GetPlayerController 0))
  (Rendering|SetVisibility (Variables|Default|GetWidget) false false))

(event Custom|ReturnHandle
  (bind _handle (Timeline|Reversed%20handle Play)
    (:Update
      (Transformation|SetWorldLocation (Variables|Default|GetHandle) (Math|Vector|Lerp(Vector) (- (Variables|Default|GetHandle1) (Variables|Default|Getdecrease)) (Variables|Default|GetHandle1) _handle) false false)
      (Transformation|SetWorldLocation (Variables|Default|GetHandle2) (Math|Vector|Lerp(Vector) (- (Variables|Default|GetHandle%282%29) (Variables|Default|Getdecrease)) (Variables|Default|GetHandle%282%29) _handle) true false))))

(event EventBeginPlay
  (Variables|Default|SetHandle1 (Transformation|GetWorldLocation (Variables|Default|GetHandle)))
  (Variables|Default|SetHandle%282%29 (Transformation|GetWorldLocation (Variables|Default|GetHandle2))))

(event Input|KeyboardEvents|E
  (params (Key :type Key%20Structure :default "None"))
  (:Pressed
    (if (not (Variables|Default|GetIsanimated?))
      (Variables|Default|SetIsanimated? true)
      (bind _handle (Timeline|Pompe%20manivelle Play)
        (:Update
          (Transformation|SetWorldLocation (Variables|Default|GetHandle) (Math|Vector|Lerp(Vector) (Variables|Default|GetHandle1) (- (Variables|Default|GetHandle1) (Variables|Default|Getdecrease)) _handle) true false)
          (Transformation|SetWorldLocation (Variables|Default|GetHandle2) (Math|Vector|Lerp(Vector) (Variables|Default|GetHandle%282%29) (- (Variables|Default|GetHandle%282%29) (Variables|Default|Getdecrease)) _handle) true false))
        (:Finished
          (CallFunction|ReturnHandle))))))

(fn ConstructionScript)