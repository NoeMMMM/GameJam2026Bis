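; BP_Water is a rising water hazard that sends the player to game over when its death plane catches them.
; On BeginPlay, two timelines run in parallel, lerping the world Z of the Water and Death components upward.
; The death plane starts far below the water and ends slightly above it.
; Its overlap with BP_FirstPersonCharacter opens the GameOver level.
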(event OnComponentBeginOverlap(Death)
  (params (OverlappedComponent :type Primitive%20Component%20Object%20Reference) (OtherActor :type Actor%20Object%20Reference) (OtherComp :type Primitive%20Component%20Object%20Reference) (OtherBodyIndex :type Integer) (bFromSweep :type Boolean) (SweepResult :type Hit%20Result%20Structure%20%28by%20ref%29))
  ;[0.15 0.15 0.15 0.5] Si DeathPlane touche le joueur alors il meurt.
  (Utilities|Casting|CastToBP_FirstPersonCharacter OtherActor)
  (Game|OpenLevel(byName) "GameOver"))

(event EventBeginPlay
  ;[0.15 0.15 0.15 0.5] Eau et DeathPlane monte
  (Utilities|FlowControl|Sequence
    (:then_0
      (bind _alpha (Timeline|EauMonte Play)
        (:Update
          (Transformation|SetWorldLocation (Variables|Default|GetWater) (Math|Vector|MakeVector 0.0 0.0 (Math|Float|Lerp -1e+01 2e+02 _alpha)) false false))))
    (:then_1
      (bind _alpha_2 (Timeline|Timeline Play)
        (:Update
          (Transformation|SetWorldLocation (Variables|Default|GetDeath) (Math|Vector|MakeVector 0.0 0.0 (Math|Float|Lerp -1e+03 2.1e+02 _alpha_2)) false false))))))

(fn ConstructionScript)