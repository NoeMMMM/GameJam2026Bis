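; Parent Blueprint for an interactable switch ("Interrupteur") that highlights when looked at and flips on interaction.
; OnLookat applies an overlay material to the pivot and switch meshes, and a short retriggerable delay clears it once the look events stop.
; OnInteract alternates a FlipFlop that plays or reverses the OnOff timeline, which lerps the pivot's pitch between two fixed angles.
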(event EventOnLookat
  (params (Actor :type Actor%20Object%20Reference))
  (if true
    (Rendering|Material|SetOverlayMaterial (Variables|Default|GetPivot1) "/Game/GameJam/Materials/M_Overlay.M_Overlay" :!class /Script/Engine.MeshComponent)
    (Utilities|FlowControl|RetriggerableDelay 0.11)
    (Rendering|Material|SetOverlayMaterial (Variables|Default|GetPivot1) 0 :!class /Script/Engine.MeshComponent)))

(event EventOnInteract
  (params (Actor :type Actor%20Object%20Reference))
  (bind _pivot1 (Variables|Default|GetPivot1))
  (bind _returnvalue (Transformation|GetSocketRotation _pivot1 "None"))
  (Utilities|FlowControl|FlipFlop
    (:A
      (Variables|Default|SetCurrentRotation (.pitch (Transformation|GetWorldRotation (Variables|Default|GetPivot1))))
      (bind _alpha (Timeline|On/Off PlayFromStart)
        (:Update
          (Transformation|SetWorldRotation (Variables|Default|GetPivot1) (Math|Rotator|MakeRotator (.roll _returnvalue) (Math|Float|Lerp -5e+01 5e+01 _alpha) (.yaw _returnvalue)) false false))))
    (:B
      (Timeline|On/Off ReverseFromEnd))))

(fn ConstructionScript)