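; BP_Valve is an interactive valve that the player turns left or right while inside its collision volume.
; Overlap begin and end enable and disable input for player 0, without checking which actor overlaps.
; Holding Left or Right plays that direction's timeline, lerping ValveCube's roll from its current value toward -360 or 360; release stops it.
; Press flags block opposing input, and the SetVisibility nodes are unwired.
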(event OnComponentBeginOverlap(ValveCollision)
  (params (OverlappedComponent :type Primitive%20Component%20Object%20Reference) (OtherActor :type Actor%20Object%20Reference) (OtherComp :type Primitive%20Component%20Object%20Reference) (OtherBodyIndex :type Integer) (bFromSweep :type Boolean) (SweepResult :type Hit%20Result%20Structure%20%28by%20ref%29))
  ;[0.15 0.15 0.15 0.5] Affiche la touche [E]
  (Input|EnableInput (Game|GetPlayerController 0)))

(event OnComponentEndOverlap(ValveCollision)
  (params (OverlappedComponent :type Primitive%20Component%20Object%20Reference) (OtherActor :type Actor%20Object%20Reference) (OtherComp :type Primitive%20Component%20Object%20Reference) (OtherBodyIndex :type Integer))
  ;[0.15 0.15 0.15 0.5] Affiche la touche [E]
  (Input|DisableInput (Game|GetPlayerController 0)))

(event Input|KeyboardEvents|E
  (params (Key :type Key%20Structure :default "None"))
  ;[0.15 0.15 0.15 0.5] La valve tourne quand [<] ou [>]
)

(event Input|KeyboardEvents|Left
  (params (Key :type Key%20Structure :default "None"))
  ;[0.15 0.15 0.15 0.5] La valve tourne quand [<] ou [>]
  (:Pressed
    (if (not (Variables|Default|GetIsPressRight))
      (Variables|Default|SetIsPressLeft true)
      (Variables|Default|SetCurrentRotation (.roll (Transformation|GetWorldRotation (Variables|Default|GetValveCube))))
      (bind _alpha (Timeline|TurnValve PlayFromStart)
        (:Update
          (Transformation|SetWorldRotation (Variables|Default|GetValveCube) (Math|Rotator|MakeRotator (Math|Float|Lerp (Variables|Default|GetCurrentRotation) -3.6e+02 _alpha) 0.0 0.0) false false)))))
  (:Released
    (Variables|Default|SetIsPressLeft false)
    (Timeline|TurnValve Stop)))

(event Input|KeyboardEvents|Right
  (params (Key :type Key%20Structure :default "None"))
  ;[0.15 0.15 0.15 0.5] La valve tourne quand [<] ou [>]
  (:Pressed
    (if (not (Variables|Default|GetIsPressLeft))
      (Variables|Default|SetIsPressRight true)
      (Variables|Default|SetCurrentRotation (.roll (Transformation|GetWorldRotation (Variables|Default|GetValveCube))))
      (bind _alpha (Timeline|Timeline PlayFromStart)
        (:Update
          (Transformation|SetWorldRotation (Variables|Default|GetValveCube) (Math|Rotator|MakeRotator (Math|Float|Lerp (Variables|Default|GetCurrentRotation) 3.6e+02 _alpha) 0.0 0.0) false false)))))
  (:Released
    (Variables|Default|SetIsPressRight false)
    (Timeline|Timeline Stop)))

(fn ConstructionScript)