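; BP_Simon runs a Simon-style memory minigame that starts when a player overlaps its box.
; Each level builds a random button sequence from its Structure entry, optionally without repeats, then plays it through recursive delayed calls.
; Linked buttons report player notes for checking; success advances the level and can flag a number display, while mistakes play errors and restart the level.
; The construction script rewrites no-repeat levels requesting more notes than buttons.
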(event OnComponentBeginOverlap(Box)
  (params (OverlappedComponent :type Primitive%20Component%20Object%20Reference) (OtherActor :type Actor%20Object%20Reference) (OtherComp :type Primitive%20Component%20Object%20Reference) (OtherBodyIndex :type Integer) (bFromSweep :type Boolean) (SweepResult :type Hit%20Result%20Structure%20%28by%20ref%29))
  (if (and (Utilities|DoesObjectImplementInterface OtherActor "/Game/GameJam/Blueprint_Interface/BPI_Player.BPI_Player_C") (not (Variables|Default|GetIsPlaying)))
    (Variables|Default|SetIsPlaying true)
    (CallFunction|StartLevel)))

(event Custom|StartLevel
  (Utilities|Array|Clear (Variables|Default|GetPlayerSequence))
  (Variables|Default|SetCurrentNote 0)
  (Variables|Default|SetIsPlayerTurn false)
  (CallFunction|MakeSimonSecquence))

(event Custom|MakeSimonSecquence
  (bind _current_level (Variables|Default|GetCurrent%20Level))
  (bind _structure (Variables|Default|GetStructure))
  (bind _output (Utilities|Array|Get(acopy) _structure _current_level))
  (bind (_numberofnote _secondbtnote _canduplicatenotes) (Utilities|Struct|BreakSimonLevel_Struct _output))
  ;[0.15 0.15 0.15 0.5] Create random sequence
  (Utilities|Array|Clear (Variables|Default|GetSimonSecquenece))
  (if (> (Utilities|Array|Length (Variables|Default|GetButton)) 0)
    (if _canduplicatenotes
      (Utilities|Array|Add (Variables|Default|GetSimonSecquenece) (Math|Random|RandomIntegerinRange 0 (Utilities|Array|LastIndex (Variables|Default|GetButton))))
      (else
        (Utilities|Array|AddUnique (Variables|Default|GetSimonSecquenece) (Math|Random|RandomIntegerinRange 0 (Utilities|Array|LastIndex (Variables|Default|GetButton))))))
    (if (< (Utilities|Array|Length (Variables|Default|GetSimonSecquenece)) _numberofnote)
      (Utilities|FlowControl|Delay 0.2)
      (CallFunction|AddAnotherNote)
      (else
        (Utilities|FlowControl|Delay 1.0)
        (CallFunction|PlaySimonSequence)))))

(event Custom|AddAnotherNote
  (bind _current_level (Variables|Default|GetCurrent%20Level))
  (bind _structure (Variables|Default|GetStructure))
  (bind _output (Utilities|Array|Get(acopy) _structure _current_level))
  (bind (_numberofnote _secondbtnote _canduplicatenotes) (Utilities|Struct|BreakSimonLevel_Struct _output))
  ;[0.15 0.15 0.15 0.5] Create random sequence
  (if (> (Utilities|Array|Length (Variables|Default|GetButton)) 0)
    (if _canduplicatenotes
      (Utilities|Array|Add (Variables|Default|GetSimonSecquenece) (Math|Random|RandomIntegerinRange 0 (Utilities|Array|LastIndex (Variables|Default|GetButton))))
      (else
        (Utilities|Array|AddUnique (Variables|Default|GetSimonSecquenece) (Math|Random|RandomIntegerinRange 0 (Utilities|Array|LastIndex (Variables|Default|GetButton))))))
    (if (< (Utilities|Array|Length (Variables|Default|GetSimonSecquenece)) _numberofnote)
      (Utilities|FlowControl|Delay 0.2)
      (CallFunction|AddAnotherNote)
      (else
        (Utilities|FlowControl|Delay 1.0)
        (CallFunction|PlaySimonSequence)))))

(event Custom|PlaySimonSequence
  (Default|PlayNote (Utilities|Array|Get(acopy) (Variables|Default|GetButton) (Utilities|Array|Get(acopy) (Variables|Default|GetSimonSecquenece) (Variables|Default|GetCurrentNote))))
  (Utilities|FlowControl|Delay (.SecondBtNote (Utilities|Struct|BreakSimonLevel_Struct (Utilities|Array|Get(acopy) (Variables|Default|GetStructure) (Variables|Default|GetCurrent%20Level)))))
  (Math|Integer|IncrementInt (Variables|Default|GetCurrentNote)
    (:%20%20
      (if (< (Variables|Default|GetCurrentNote) (Utilities|Array|Length (Variables|Default|GetSimonSecquenece)))
        (CallFunction|PlaySimonSequence)
        (Variables|Default|SetIsPlayerTurn true)))))

(event Custom|PlayerPlayedNote
  (params (Note :type Integer))
  (Variables|Default|SetIsPlayerTurn false)
  (bind _returnvalue (Utilities|Array|Add (Variables|Default|GetPlayerSequence) Note))
  (for _array_element (Variables|Default|GetPlayerSequence)
    (Development|PrintString (Utilities|String|ToString(Integer) _array_element) false false)
    (if (== Note (Utilities|Array|Get(acopy) (Variables|Default|GetSimonSecquenece) _returnvalue))
      (Default|PlayNote (Utilities|Array|Get(acopy) (Variables|Default|GetButton) Note))
      (if (>= (Utilities|Array|Length (Variables|Default|GetPlayerSequence)) (Utilities|Array|Length (Variables|Default|GetSimonSecquenece)))
        (if (< (Variables|Default|GetCurrent%20Level) (Utilities|Array|LastIndex (Variables|Default|GetStructure)))
          (CallFunction|ShowNumber)
          (Math|Integer|IncrementInt (Variables|Default|GetCurrent%20Level)
            (:%20%20
              (Utilities|FlowControl|Delay 1.0)
              (CallFunction|StartLevel))))
        (else
          (Variables|Default|SetIsPlayerTurn true)))
      (else
        (for _array_element_2 (Variables|Default|GetButton)
          (Default|PlayError _array_element_2))
        (Utilities|FlowControl|Delay 2.0)
        (CallFunction|StartLevel)))))

(event Custom|ShowNumber
  (if (>= (Variables|Default|GetCurrent%20Level) 2)
    (Variables|Default|SetShowNumberOnScreen true)))

(event EventBeginPlay
  (for _array_element (Variables|Default|GetButton)
    (Utilities|IsValid _array_element
      (:Is%20Valid
        (Variables|/Game/GameJam/Blueprint/BP_Button.BP_Button_C|SetSimonMain_Ref _array_element self)))))

(fn ConstructionScript
  (for (_array_element _array_index) (Variables|Default|GetStructure)
    (if (not (.CanDuplicateNotes (Utilities|Struct|BreakSimonLevel_Struct _array_element)))
      (if (> (.NumberOfNote (Utilities|Struct|BreakSimonLevel_Struct _array_element)) (Utilities|Array|Length (Variables|Default|GetButton)))
        (bind _structout (Utilities|Struct|SetmembersinSimonLevel_Struct _array_element))
        (Utilities|Array|SetArrayElem (Variables|Default|GetStructure) _array_index _structout)))))