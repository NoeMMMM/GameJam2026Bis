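; BP_Button is one button of a Simon-style memory game, with its own color, sound and index.
; Interacting during the player's turn reports its index to SimonMainRef, and looking at it briefly applies a highlight overlay via a retriggerable delay.
; PlayNote plays its sound and brightens a dynamic material created in the construction script.
; PlayError temporarily swaps in a red flash and failure sound, then restores both.
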(event Custom|Play%20Note
  (Audio|Components|Audio|Play (Variables|Default|GetAudio) 0.0)
  (Rendering|Material|SetScalarParameterValue (Variables|Default|GetDyn%20Mat) "Intensity" 2.5 :!class /Script/Engine.MaterialInstanceDynamic)
  (Utilities|FlowControl|Delay 0.6)
  (Audio|Components|Audio|Stop (Variables|Default|GetAudio))
  (Rendering|Material|SetScalarParameterValue (Variables|Default|GetDyn%20Mat) "Intensity" 1.0 :!class /Script/Engine.MaterialInstanceDynamic))

(event Custom|PlayError
  (Audio|Components|Audio|SetSound (Variables|Default|GetAudio) "/Game/GameJam/Audio/Son_Echec_1.Son_Echec_1")
  (Audio|Components|Audio|Play (Variables|Default|GetAudio) 0.0)
  (Rendering|Material|SetVectorParameterValue (Variables|Default|GetDyn%20Mat) "Color" "(R=1.000000,G=0.000000,B=0.000000,A=1.000000)" :!class /Script/Engine.MaterialInstanceDynamic)
  (Rendering|Material|SetScalarParameterValue (Variables|Default|GetDyn%20Mat) "Intensity" 2.5 :!class /Script/Engine.MaterialInstanceDynamic)
  (Utilities|FlowControl|Delay 0.6)
  (Audio|Components|Audio|Stop (Variables|Default|GetAudio))
  (Rendering|Material|SetScalarParameterValue (Variables|Default|GetDyn%20Mat) "Intensity" 1.0 :!class /Script/Engine.MaterialInstanceDynamic)
  (Rendering|Material|SetVectorParameterValue (Variables|Default|GetDyn%20Mat) "Color" (Variables|Default|GetColor) :!class /Script/Engine.MaterialInstanceDynamic)
  (Audio|Components|Audio|SetSound (Variables|Default|GetAudio) (Variables|Default|GetSound)))

(event EventBeginPlay
  (Audio|Components|Audio|SetSound (Variables|Default|GetAudio) (Variables|Default|GetSound)))

(event Collision|EventActorBeginOverlap
  (params (OtherActor :type Actor%20Object%20Reference)))

(event EventTick
  (params (DeltaSeconds :type Float%20%28single-precision%29)))

(event EventOnInteract
  (params (Actor :type Actor%20Object%20Reference))
  (if (Utilities|DoesObjectImplementInterface Actor "/Game/GameJam/Blueprint_Interface/BPI_Player.BPI_Player_C")
    (bind _simonmain_ref (Variables|Default|GetSimonMain_Ref)
      (:then
        (if (Variables|/Game/GameJam/Blueprint/BP_Simon.BP_Simon_C|GetIsPlayerTurn _simonmain_ref)
          (Default|PlayerPlayedNote _simonmain_ref (Variables|Default|GetIndex))))
      (:else))))

(event EventOnLookat
  (params (Actor :type Actor%20Object%20Reference))
  (bind _simonmain_ref (Variables|Default|GetSimonMain_Ref)
    (:then
      (if (Variables|/Game/GameJam/Blueprint/BP_Simon.BP_Simon_C|GetIsPlayerTurn _simonmain_ref)
        (Rendering|Material|SetOverlayMaterial (Variables|Default|GetStaticMesh) "/Game/GameJam/Materials/M_Overlay.M_Overlay" :!class /Script/Engine.MeshComponent)
        (Utilities|FlowControl|RetriggerableDelay 0.11)
        (Rendering|Material|SetOverlayMaterial (Variables|Default|GetStaticMesh) 0 :!class /Script/Engine.MeshComponent)))
    (:else)))

(fn ConstructionScript
  (bind _returnvalue (Rendering|Material|CreateDynamicMaterialInstance (Variables|Default|GetStaticMesh) 0 "/Game/GameJam/Materials/M_Color.M_Color" "None" :!class /Script/Engine.PrimitiveComponent))
  (bind _output_get (Variables|Default|SetDyn%20Mat _returnvalue))
  (Rendering|Material|SetVectorParameterValue _output_get "Color" (Variables|Default|GetColor) :!class /Script/Engine.MaterialInstanceDynamic))