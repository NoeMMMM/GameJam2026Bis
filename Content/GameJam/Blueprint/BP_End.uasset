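; BP_End is an end-point actor that times a run and displays the elapsed time on a widget component.
; While StopTimer is true, which counterintuitively means running, Tick accumulates delta seconds into Timer and sets the widget visible every frame.
; Any overlap with its Box clears StopTimer and writes the formatted time into the WBP_End text block.
; Nothing in this Blueprint sets StopTimer to true.
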(event OnComponentBeginOverlap(Box)
  (params (OverlappedComponent :type Primitive%20Component%20Object%20Reference) (OtherActor :type Actor%20Object%20Reference) (OtherComp :type Primitive%20Component%20Object%20Reference) (OtherBodyIndex :type Integer) (bFromSweep :type Boolean) (SweepResult :type Hit%20Result%20Structure%20%28by%20ref%29))
  (Variables|Default|SetStop%20timer false)
  (bind _aswbp_end (Utilities|Casting|CastToWBP_End (UserInterface|GetWidget (Variables|Default|GetWidget))))
  (Variables|/Script/UMG.TextBlock|SetText (Variables|/Game/GameJam/Widget/WBP_End.WBP_End_C|GetTextBlock_1 _aswbp_end) (Utilities|Text|ToText(String) (Class|KismetStringLibrary|TimeSecondstoString (Variables|Default|GetTimer)))))

(event EventTick
  (params (DeltaSeconds :type Float%20%28single-precision%29))
  (if (Variables|Default|GetStop%20timer)
    (Variables|Default|SetTimer (+ (Variables|Default|GetTimer) (Utilities|Time|GetWorldDeltaSeconds)))
    (Widget|SetVisibility (UserInterface|GetWidget (Variables|Default|GetWidget)) "Visible")))

(fn ConstructionScript)